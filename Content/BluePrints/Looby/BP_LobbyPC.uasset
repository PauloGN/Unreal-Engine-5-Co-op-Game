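; Lobby player controller that manages the local player's lobby UI and their name and ready status.
; On BeginPlay, the local controller shows the cursor, creates the lobby widget and submits an empty name.
; Name changes and ready toggles update its player info struct and pass the controller to BP_GameModeLobby, with a delayed retry event available.
; OnStartMath shows the widget's loading screen and disables input.
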(event `self.ReceiveBeginPlay`
  (`self.SetUp`))

(event `TryAgain`
  ;[1 1 1] Try Update lobby info in case of fail
  (`KismetSystemLibrary.Delay` 0.2)
  (bind _asbp_game_mode_lobby (cast `/Game/BluePrints/Looby/BP_GameModeLobby` (`GameplayStatics.GetGameMode`)))
  (`/Game/BluePrints/Looby/BP_GameModeLobby.UpdatePlayerLobbyInfo` _asbp_game_mode_lobby self))

(event `SetPlayerNameOnServer`
  (params (PlayerName :type Text))
  ;[1 1 1] Set Player name on lobby platform
  (setmembers `/Game/BluePrints/Looby/S_PlayerLobbyInfo` :`StructRef` (`self.PlayerInfoLobbyPC`) :`PLayerName` PlayerName)
  (bind _asbp_game_mode_lobby (cast `/Game/BluePrints/Looby/BP_GameModeLobby` (`GameplayStatics.GetGameMode`)))
  (`/Game/BluePrints/Looby/BP_GameModeLobby.UpdatePlayerLobbyInfo` _asbp_game_mode_lobby self))

(event `ToggleReadyStatusOnServer`
  (bind _playerinfolobbypc (`self.PlayerInfoLobbyPC`))
  ;[1 1 1] Ready and not Ready Status
  (setmembers `/Game/BluePrints/Looby/S_PlayerLobbyInfo` :`StructRef` _playerinfolobbypc :`bReady` (not (`.bReady_8_EE805FEA4C9B0A1B294F2C82D4FBFAC3` (break `/Game/BluePrints/Looby/S_PlayerLobbyInfo` _playerinfolobbypc))))
  (bind _asbp_game_mode_lobby (cast `/Game/BluePrints/Looby/BP_GameModeLobby` (`GameplayStatics.GetGameMode`)))
  (`/Game/BluePrints/Looby/BP_GameModeLobby.UpdatePlayerLobbyInfo` _asbp_game_mode_lobby self))

(event `OnStartMath`
  ;[1 1 1] Blur-loading effect
  (`/Game/BluePrints/Looby/WPB_LobbyUI.ShowLoadingScreen` (`self.LobbyUI_REF`))
  (`self.DisableInput` self))

(fn `SetUp`
  (if (`self.IsLocalController`)
    (set `self.bShowMouseCursor` true)
    (`WidgetBlueprintLibrary.SetInputMode_GameAndUIEx` self null "DoNotLock" false)
    (bind _returnvalue (`|CreateWidget` "/Game/BluePrints/Looby/WPB_LobbyUI.WPB_LobbyUI_C"))
    (bind _output_get (set `self.LobbyUI_REF` _returnvalue))
    (`UserWidget.AddToViewport` _output_get 0)
    (`self.SetPlayerNameOnServer` "")))

(fn `UserConstructionScript`)