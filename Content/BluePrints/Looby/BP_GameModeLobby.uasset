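; Lobby game mode that seats connected players on BP_LoobyPlayerPlatform actors and tracks their ready state.
; Platforms are gathered in order by numeric tag; on login or logout, a delay-polling macro waits for setup, then platforms spawn characters for new players and clear departed ones.
; Lobby info updates go to the player's platform, then set an all-ready flag on the first local controller's lobby UI.
; It also notifies controllers before match start or session cancel, which destroys the server.
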(event `self.ReceiveBeginPlay`
  (`self.SetupPlatforms`))

(event `self.K2_PostLogin`
  (params (NewPlayer :type "PlayerController Object Reference"))
  (`KismetArrayLibrary.Array_Add` (`self.PCs`) NewPlayer)
  (`self.IFPlatformSetUpIsdone` :!label _label
    (:`true`
      (`self.UpdatePlayersOnPlatforms`))))

(event `self.K2_OnLogout`
  (params (ExitingController :type "Controller Object Reference"))
  (bind _asplayer_controller (cast `PlayerController` ExitingController))
  (`KismetArrayLibrary.Array_RemoveItem` (`self.PCs`) _asplayer_controller)
  (goto _label))

(fn `BeforeStartMatch`
  (for _array_element (`self.PCs`)
    (bind _asbp_lobby_pc (cast `/Game/BluePrints/Looby/BP_LobbyPC` _array_element))
    (`/Game/BluePrints/Looby/BP_LobbyPC.OnStartMath` _asbp_lobby_pc)))

(fn `CancelSession`
  (bind _returnvalue (subsystem `MultiplayerSessionsSubsystem`))
  (for _array_element (`self.PCs`)
    (bind _asbp_lobby_pc (cast `/Game/BluePrints/Looby/BP_LobbyPC` _array_element))
    (`/Game/BluePrints/Looby/BP_LobbyPC.OnStartMath` _asbp_lobby_pc)
    (`/Engine/EditorBlueprintResources/StandardMacros.IsValid` _returnvalue
      (:`Is Valid`
        (`MultiplayerSessionsSubsystem.DestroyLastServer` _returnvalue)))))

(fn `CheckIfEnoughPlayersAreReady`
  (locals (bAllPlayersReady :type Boolean))
  (set `local.bAllPlayersReady` true)
  (for _array_element (`self.PCs`)
    (bind _asbp_lobby_pc (cast `/Game/BluePrints/Looby/BP_LobbyPC` _array_element))
    (if (not (`.bReady_8_EE805FEA4C9B0A1B294F2C82D4FBFAC3` (break `/Game/BluePrints/Looby/S_PlayerLobbyInfo` (`/Game/BluePrints/Looby/BP_LobbyPC.PlayerInfoLobbyPC` _asbp_lobby_pc))))
      (set `local.bAllPlayersReady` false)))
  (bind _asbp_lobby_pc_2 (cast `/Game/BluePrints/Looby/BP_LobbyPC` (`GameplayStatics.GetPlayerController` 0)))
  (set `/Game/BluePrints/Looby/WPB_LobbyUI.bEnoughPlayersReady` (`local.bAllPlayersReady`) (`/Game/BluePrints/Looby/BP_LobbyPC.LobbyUI_REF` _asbp_lobby_pc_2)))

(fn `SetupPlatforms`
  (bind _outactors (`GameplayStatics.GetAllActorsOfClass` "/Game/BluePrints/Looby/BP_LoobyPlayerPlatform.BP_LoobyPlayerPlatform_C"))
  (for _index (range (+ (`KismetArrayLibrary.Array_LastIndex` _outactors) 1))
    (bind _outactors_2 (`GameplayStatics.GetAllActorsOfClassWithTag` "/Game/BluePrints/Looby/BP_LoobyPlayerPlatform.BP_LoobyPlayerPlatform_C" (`KismetStringLibrary.Conv_StringToName` (`KismetStringLibrary.Conv_IntToString` _index))))
    (`KismetArrayLibrary.Array_Add` (`self.LobbyPlayerPlatform`) (`|GetArrayItem` _outactors_2)))
  (set `self.bPlayerPlatformDone` true))

(fn `UpdatePlayerLobbyInfo`
  (params (RequestingPC :type "PlayerController Object Reference"))
  (bind _asbp_lobby_pc (cast `/Game/BluePrints/Looby/BP_LobbyPC` (`local.RequestingPC`) :!pure true))
  (bind (_playerinfolobbypc_pc _playerinfolobbypc_playername _playerinfolobbypc_bready) (break `/Game/BluePrints/Looby/S_PlayerLobbyInfo` (`/Game/BluePrints/Looby/BP_LobbyPC.PlayerInfoLobbyPC` _asbp_lobby_pc)))
  (bind _playerstate (`Controller.PlayerState` _asbp_lobby_pc))
  (for _array_element (`self.LobbyPlayerPlatform`)
    (if (== RequestingPC (`/Game/BluePrints/Looby/BP_LoobyPlayerPlatform.PC` _array_element))
      (`/Game/BluePrints/Looby/BP_LoobyPlayerPlatform.UpdateLobbyInfo` _array_element (make `/Game/BluePrints/Looby/S_PlayerLobbyInfo` (`local.RequestingPC`) (`KismetTextLibrary.Conv_StringToText` (`PlayerState.GetPlayerName` _playerstate)) _playerinfolobbypc_bready _playerstate))
      (`self.CheckIfEnoughPlayersAreReady`)
      (return)))
  (`/Game/BluePrints/Looby/BP_LobbyPC.TryAgain` (cast `/Game/BluePrints/Looby/BP_LobbyPC` (`local.RequestingPC`) :!pure true)))

(fn `UpdatePlayersOnPlatforms`
  (locals (Loop_PC_alreadyAdded :type Boolean))
  ;[1 1 1] Is PC already added to the platform
  (for _array_element (`self.PCs`)
    (set `local.Loop_PC_alreadyAdded` false)
    (for _array_element_2 (`self.LobbyPlayerPlatform`)
      (`/Engine/EditorBlueprintResources/StandardMacros.IsValid` _array_element_2
        (:`Is Valid`
          (if (== (`/Game/BluePrints/Looby/BP_LoobyPlayerPlatform.PC` _array_element_2) _array_element)
            (set `local.Loop_PC_alreadyAdded` true)
            (break)))))
    ;[1 1 1] Add pc to platform
    (if (not (`local.Loop_PC_alreadyAdded`))
      (for _array_element_3 (`self.LobbyPlayerPlatform`)
        (`/Engine/EditorBlueprintResources/StandardMacros.IsValid` (`/Game/BluePrints/Looby/BP_LoobyPlayerPlatform.PC` _array_element_3)
          (:`Is Not Valid`
            (`/Game/BluePrints/Looby/BP_LoobyPlayerPlatform.SpawnCharacter` _array_element_3 _array_element)
            (break))))))
  ;[1 1 1] Remove disconected players from platform
  (for _array_element_4 (`self.LobbyPlayerPlatform`)
    (`/Engine/EditorBlueprintResources/StandardMacros.IsValid` _array_element_4
      (:`Is Valid`
        (if (not (`KismetArrayLibrary.Array_Contains` (`self.PCs`) (`/Game/BluePrints/Looby/BP_LoobyPlayerPlatform.PC` _array_element_4)))
          (`/Engine/EditorBlueprintResources/StandardMacros.IsValid` _array_element_4
            (:`Is Valid`
              (`/Game/BluePrints/Looby/BP_LoobyPlayerPlatform.Clear` _array_element_4))))))))

(fn `UserConstructionScript`)