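; Lobby platform actor that displays a player's character and lobby info for a given player controller.
; SpawnCharacter replaces any existing character with a new BP_ThirdPersonCharacter at the PlayerTransform component.
; UpdateLobbyInfo sets PlayerLobbyinfo, whose RepNotify updates and shows the WBP_LobbyInfomenu widget, retrying on a short timer until the widget exists.
; Clear resets the controller reference and, if a character exists, destroys the platform actor itself.
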(event `SpawnCharacter`
  (params (PC :type "PlayerController Object Reference"))
  (bind _playercharacter (`self.PlayerCharacter`))
  (set `self.PC` PC)
  (`/Engine/EditorBlueprintResources/StandardMacros.IsValid` _playercharacter
    (:`Is Valid`
      (`self.K2_DestroyActor` _playercharacter))
    (:`Is Not Valid`
      _))
  (bind _returnvalue (`|SpawnActorFromClass` "/Game/ThirdPerson/Blueprints/BP_ThirdPersonCharacter.BP_ThirdPersonCharacter_C" (`SceneComponent.K2_GetComponentToWorld` (`self.playerTransform`)) "Undefined" "MultiplyWithRoot" null null))
  (bind _output_get (set `self.PlayerCharacter` _returnvalue))
  (cast `/Game/ThirdPerson/Blueprints/BP_ThirdPersonCharacter` _output_get))

(event `Clear`
  (set `self.PC` null)
  (`/Engine/EditorBlueprintResources/StandardMacros.IsValid` (`self.PlayerCharacter`)
    (:`Is Valid`
      (`self.K2_DestroyActor`)
      (set `self.PC` null))))

(fn `OnRep_PlayerLobbyinfo`
  (bind _returnvalue (`WidgetComponent.GetWidget` (`self.WidgetLobby`)))
  (`/Engine/EditorBlueprintResources/StandardMacros.IsValid` _returnvalue
    (:`Is Valid`
      (bind _aswbp_lobby_infomenu (cast `/Game/BluePrints/Looby/WBP_LobbyInfomenu` _returnvalue))
      (`/Game/BluePrints/Looby/WBP_LobbyInfomenu.Update` _aswbp_lobby_infomenu (`self.PlayerLobbyinfo`))
      (`SceneComponent.SetVisibility` (`self.WidgetLobby`) true false))
    (:`Is Not Valid`
      (`KismetSystemLibrary.K2_SetTimer` null "OnRep_PlayerLobbyinfo" 0.1))))

(fn `UpdateLobbyInfo`
  (params (PlayerLobbyinfo :type "/Game/BluePrints/Looby/S_PlayerLobbyInfo Structure"))
  (set `self.PlayerLobbyinfo` PlayerLobbyinfo))

(fn `UserConstructionScript`)