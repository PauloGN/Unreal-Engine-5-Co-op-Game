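; BP_InGameGameMode is the in-game game mode that spawns each player as their selected character.
; It overrides GetDefaultPawnClassForController to look up the player's name from PlayerState in the SelectedCharactersOfAllPlayers map on BP_MyGameInstance.
; A found entry becomes the pawn class; otherwise the parent implementation's default is used.
; The event graph and construction script hold no logic.
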(event `self.ReceiveBeginPlay`)

(fn `GetDefaultPawnClassForController`
  (params (InController :type "Controller Object Reference"))
  (returns (ReturnValue :type "Object Class Reference"))
  (locals (SpawnedChar :type "Object Class Reference"))
  (bind (_value _returnvalue) (`BlueprintMapLibrary.Map_Find` (`/Game/BluePrints/BP_MyGameInstance.SelectedCharactersOfAllPlayers` (cast `/Game/BluePrints/BP_MyGameInstance` (`GameplayStatics.GetGameInstance`) :!pure true)) (`PlayerState.GetPlayerName` (`Controller.PlayerState` (`local.InController`)))))
  (bind _returnvalue_2 (`parent.GetDefaultPawnClassForController` InController))
  (if _returnvalue
    (set `local.SpawnedChar` _value)
    (else
      (set `local.SpawnedChar` _returnvalue_2)))
  (return (`local.SpawnedChar`)))

(fn `UserConstructionScript`)