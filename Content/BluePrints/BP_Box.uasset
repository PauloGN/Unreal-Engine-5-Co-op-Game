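; BP_Box is a debug actor that displays network authority and a float variable, ReplicatedFloat, on text components.
; On BeginPlay it checks HasAuthority and sets AuthorityText to show whether this instance has authority.
; Every Tick it writes the current ReplicatedFloat value to ReplicatedFloatText; nothing in these graphs changes that value.
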(event `self.ReceiveBeginPlay`
  (if (`self.HasAuthority`)
    (`TextRenderComponent.K2_SetText` (`self.Authority Text`) (`KismetTextLibrary.Conv_StringToText` "HasAuthority"))
    (else
      (`TextRenderComponent.K2_SetText` (`self.Authority Text`) (`KismetTextLibrary.Conv_StringToText` "No authority")))))

(event `self.ReceiveTick`
  (params (DeltaSeconds :type "Float (single-precision)"))
  (`TextRenderComponent.K2_SetText` (`self.ReplicatedFloatText`) (`KismetTextLibrary.Conv_StringToText` (`KismetStringLibrary.Concat_StrStr` "Replicated Float calling: " (`KismetStringLibrary.Conv_DoubleToString` (`self.replicatedFloat`))))))

(fn `UserConstructionScript`)