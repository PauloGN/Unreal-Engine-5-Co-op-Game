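; BP_Box is a multiplayer test actor that shows authority and replicated values through text components.
; BeginPlay labels whether the instance has authority and, only with authority, calls OnRepCountingDownFloat, whose body is not shown.
; Tick refreshes the replicated float and countdown time texts every frame.
; A RepNotify on ReplicatedBool prints a notice and the new value to screen.
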(event `self.ReceiveBeginPlay`
  ;[0.1874 0.2705 1] Full Blueprint implementation Dealing with the Authority text.
  (if (`self.HasAuthority`)
    (`TextRenderComponent.K2_SetText` (`self.Authority Text`) (`KismetTextLibrary.Conv_StringToText` "HasAuthority"))
    (`self.OnRep_CountingDownFloat`)
    (else
      (`TextRenderComponent.K2_SetText` (`self.Authority Text`) (`KismetTextLibrary.Conv_StringToText` "No authority")))))

(event `self.ReceiveTick`
  (params (DeltaSeconds :type "Float (single-precision)"))
  ;[0.2883 0.212 1] Mixed Implementation
  (`TextRenderComponent.K2_SetText` (`self.ReplicatedFloatText`) (`KismetTextLibrary.Conv_StringToText` (`KismetStringLibrary.Concat_StrStr` "Replicated Float calling: " (`KismetStringLibrary.Conv_DoubleToString` (`self.replicatedFloat`)))))
  (`TextRenderComponent.K2_SetText` (`self.CountingDownText`) (`KismetTextLibrary.Conv_StringToText` (`KismetStringLibrary.Concat_StrStr` "Time: " (`KismetStringLibrary.Conv_DoubleToString` (`self.CountingDownFloat`))))))

(fn `OnRep_replicatedBool`
  ;[0.7197 0 1] This will altomatically show the server or client ID
  (`KismetSystemLibrary.PrintString` "On replicated bool" true true (struct :`R` 0.31529 :`B` 1.0 :`A` 1.0) 20.0)
  (`KismetSystemLibrary.PrintString` (`KismetStringLibrary.Conv_BoolToString` (`self.replicatedBool`))))

(fn `UserConstructionScript`)