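; BP_FireKey is a fire gameplay object with a shadow light meant to wander like flickering firelight and a fire cue.
; Each Tick interpolates the light toward a fresh random point in a box around its starting height, though VInterpTo shows no delta time input.
; When IsFireOn is true, a DoOnce activates Fire01Cue a single time; this graph never sets that flag.
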(event `self.ReceiveBeginPlay`
  ;[1 1 1] Smoke treatment
  (set `self.InitalLoc` (.location (`SceneComponent.GetRelativeTransform` (`self.ShadowedLight`)))))

(event `self.ReceiveTick`
  (params (DeltaSeconds :type "Float (single-precision)"))
  (bind _shadowedlight (`self.ShadowedLight`))
  ;[1 1 1] Smoke treatment
  (`SceneComponent.K2_SetRelativeLocation` _shadowedlight (`KismetMathLibrary.VInterpTo` (`SceneComponent.RelativeLocation` _shadowedlight) (`KismetMathLibrary.RandomPointInBoundingBox` (`KismetMathLibrary.MakeVector` 0.0 0.0 (.z (`self.InitalLoc`))) (`KismetMathLibrary.MakeVector` 150.0 150.0 40.0)) 0.0 1.5) false false)
  (if (`self.bIsFireOn`)
    (`/Engine/EditorBlueprintResources/StandardMacros.DoOnce` false
      (:`Completed`
        (`ActorComponent.Activate` (`self.Fire01_Cue`) false)))))

(fn `UserConstructionScript`)